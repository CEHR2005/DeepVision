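; Sonar sphere that orbits the VR pawn like a radar sweep and pings on Pistol actors it detects.
; A looping timer moves it around the player, while Tick box-traces outward through it with a tall, thin box.
; A hit locks the sphere, plays audio pitched by distance and prints debug info; timers resume movement, then re-enable detection.
; An input action toggles orbit pause; left grab has no effect.
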(event `self.ReceiveBeginPlay`
  (`KismetSystemLibrary.K2_SetTimer` null "Update Rotation" 0.05 true)
  (bind _outactors (`GameplayStatics.GetAllActorsOfClass` "/Game/VRTemplate/Blueprints/VRPawn.VRPawn_C"))
  (set `self.MainActor` (`|GetArrayItem` _outactors))
  (`self.EnableInput` (`GameplayStatics.GetPlayerController` 0)))

(event `self.ReceiveTick`
  (params (DeltaSeconds :type "Float (single-precision)"))
  (bind (_outhits _returnvalue) (`KismetSystemLibrary.BoxTraceMultiForObjects` :`Start` (`SceneComponent.K2_GetComponentLocation` (`Actor.RootComponent` (`self.MainActor`))) :`End` (+ (`self.K2_GetActorLocation`) (* (`KismetMathLibrary.Normal` (- (`self.K2_GetActorLocation`) (`SceneComponent.K2_GetComponentLocation` (`Actor.RootComponent` (`self.MainActor`))))) (2000.0 2000.0 0.0))) :`HalfSize` (0.0 0.0 10000.0) :`ObjectTypes` (`|MakeArray` "ObjectTypeQuery4" :!type "EObjectTypeQuery Enum") :`DrawDebugType` "ForOneFrame"))
  (set `self.hitCondition` _returnvalue)
  (for _array_element _outhits
    (bind (_bblockinghit _binitialoverlap _time _distance _location _impactpoint _normal _impactnormal _physmat _hitactor) (`GameplayStatics.BreakHitResult` _array_element))
    (set `self.hitActor` _hitactor)
    (set `self.hitDistance` (`KismetMathLibrary.VSize` (- (`SceneComponent.K2_GetComponentLocation` (`Actor.RootComponent` (`self.MainActor`))) _location)))
    (if (`self.hitCondition`)
      (cast `/Game/VRTemplate/Blueprints/Pistol` (`self.hitActor`))
      (if (`self.WasLocked`)
        _
        (elif (not (`self.Locked`))
          (set `self.Locked` true)
          (set `self.Currect item` (`self.hitActor`))
          (`KismetSystemLibrary.K2_SetTimer` null "ResumeMovement" 1.0)
          (`AudioComponent.SetPitchMultiplier` (`self.Audio`) (`KismetMathLibrary.SafeDivide` 200.0 (`self.hitDistance`)))
          (`AudioComponent.Play` (`self.Audio`) 0.0)
          (`KismetSystemLibrary.PrintString` (`KismetSystemLibrary.GetDisplayName` (`self.hitActor`)) true true (struct :`G` 0.66 :`B` 1.0 :`A` 1.0) 4.0)
          (`KismetSystemLibrary.PrintString` (`KismetStringLibrary.Conv_DoubleToString` (`self.hitDistance`))))))))

(event `LockedItemInfo`
  (if (`self.Locked`)
    (`KismetSystemLibrary.PrintString` (`KismetStringLibrary.Conv_ObjectToString` (`self.Currect item`)))
    (else
      (`KismetSystemLibrary.PrintString` "Ничего нет"))))

(event `EnhancedInput|/Game/IA_VRSphere_Delay`
  (params (ActionValue :type Boolean) (ElapsedSeconds :type "Float (double-precision)") (TriggeredSeconds :type "Float (double-precision)") (InputAction :type "InputAction Object Reference" :default "/Game/IA_VRSphere_Delay.IA_VRSphere_Delay"))
  (:`Started`
    (set `self.delayed` (not (`self.delayed`)))))

(event `EnhancedInput|/Game/VRTemplate/Input/Actions/IA_Grab_Left`
  (params (ActionValue :type "Float (double-precision)") (ElapsedSeconds :type "Float (double-precision)") (TriggeredSeconds :type "Float (double-precision)") (InputAction :type "InputAction Object Reference" :default "/Game/VRTemplate/Input/Actions/IA_Grab_Left.IA_Grab_Left"))
  (:`Triggered`
    (if (or (`self.Locked`) (`self.delayed`))
      _)))

(fn `MakeVectorFromAngle`
  (params (A :type "Float (double-precision)"))
  (returns (ReturnValue :type "Vector Structure"))
  (bind _radius (`self.Radius`))
  (return (`KismetMathLibrary.MakeVector` (+ (.x (`SceneComponent.K2_GetComponentLocation` (`Actor.RootComponent` (`self.MainActor`)))) (* _radius (`KismetMathLibrary.Cos` A))) (+ (.y (`SceneComponent.K2_GetComponentLocation` (`Actor.RootComponent` (`self.MainActor`)))) (* (`KismetMathLibrary.Sin` A) _radius)) 100.0)))

(fn `ResumeMovement`
  (set `self.Locked` false)
  (set `self.WasLocked` true)
  (`KismetSystemLibrary.K2_SetTimer` null "Unlock" 1.0))

(fn `Unlock`
  (set `self.WasLocked` false)
  (set `self.Currect item` null))

(fn `Update Rotation`
  (bind _rotationspeed (`self.RotationSpeed`))
  (if (and (not (`self.Locked`)) (not (`self.delayed`)))
    (if (not (== _rotationspeed 0.0))
      (bind _output_get (set `self.Angle` (+ _rotationspeed (`self.Angle`))))
      (bind _returnvalue (`self.MakeVectorFromAngle` _output_get))
      (`self.K2_SetActorLocation` _returnvalue))))

(fn `UserConstructionScript`)